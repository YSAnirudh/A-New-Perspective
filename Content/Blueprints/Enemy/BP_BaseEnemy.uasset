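; BP_BaseEnemy is a base enemy Blueprint whose death can trigger post-fight world changes.
; On BeginPlay it finds and caches the level's BP_AfterBossBattle actor as BossTrigger.
; OnDeath tells that trigger to bring the tiles down if MakesTilesComeDown is set.
; Otherwise, a boss looks up BP_Treasure and makes its treasure takeable, so the tile flag takes precedence over the boss unlock.
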(event EventBeginPlay
  (bind _returnvalue (Actor|GetActorOfClass "/Game/Blueprints/LevelScripts/BP_AfterBossBattle.BP_AfterBossBattle_C"))
  (Variables|Default|SetBossTrigger _returnvalue))

(event Collision|EventActorBeginOverlap
  (params (OtherActor :type Actor%20Object%20Reference)))

(event EventTick
  (params (DeltaSeconds :type Float%20%28single-precision%29)))

(event EventOnDeath
  (bind _bosstrigger (Variables|Default|GetBossTrigger))
  (if (Variables|Default|GetbMakesTilesComeDown)
    (Utilities|IsValid _bosstrigger
      (:Is%20Valid
        (Class|AfterBossBattle|GettheTilesDownNow _bosstrigger)))
    (elif (Variables|Default|GetbIsBoss)
      (bind _returnvalue (Actor|GetActorOfClass "/Game/Blueprints/Pickups/BP_Treasure.BP_Treasure_C"))
      (Variables|/Script/ANewPerspective.Treasure|SetbCanTakeTreasure _returnvalue true))))

(fn ConstructionScript)